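; Enemy patroller that holds a pistol and throws pistol projectiles when it sees the player.
; On sight it turns to face the player and, if SpawnProjectile is set, launches a spinning pistol with sound and animation.
; Overlapping a Throwable_Pistol destroys it instantly with an explosion.
; Three patrol points are cached and one picked randomly at start, but the timeline-driven AIMoveTo patrol is disconnected and never runs.
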(event OnSeePawn(PawnSensing)
  (params (Pawn :type Pawn%20Object%20Reference))
  ;[1 1 1] Move and Shoot Logic
  (bind _asplayer_character (Utilities|Casting|CastToPlayerCharacter Pawn))
  (Utilities|FlowControl|Sequence
    (:then_0
      (Transformation|SetActorRotation (Math|Rotator|FindLookatRotation (Transformation|GetActorLocation) (Transformation|GetActorLocation _asplayer_character))))
    (:then_1
      (if (Variables|Default|GetSpawnProjectile)
        (bind _returnvalue (Game|SpawnActorfromClass "/Game/Guns/Throwable_Pistol_ENEMY.Throwable_Pistol_ENEMY_C" (Transformation|GetWorldTransform (Variables|Default|GetGunSpawnLocation)) "Undefined" 0 0))
        (Physics|AddImpulse (Variables|/Game/Guns/Throwable_Pistol_ENEMY.Throwable_Pistol_ENEMY_C|GetStaticMesh _returnvalue) (* (Math|Vector|GetForwardVector (Variables|Character|GetMesh)) 2.5e+03) "None" true)
        (Class|PrimitiveComponent|AddAngularImpulse (Variables|/Game/Guns/Throwable_Pistol_ENEMY.Throwable_Pistol_ENEMY_C|GetStaticMesh _returnvalue) (* (Math|Random|RandomUnitVector) 3e+01) "None" true)
        (Audio|PlaySoundatLocation "/Game/Sounds/Sound_Cues/Throw_Enemy.Throw_Enemy" (Transformation|GetActorLocation))
        (Components|Animation|PlayAnimation (Variables|Character|GetMesh) "/Game/PlayerCharacter/Animation/Animations/throwing.throwing" false)))))

(event Collision|EventActorBeginOverlap
  (params (OtherActor :type Actor%20Object%20Reference))
  (bind _returnvalue (Transformation|GetActorLocation))
  ;[1 1 1] Dies If Hit [CHANGE TO TAKE DMG]
  (Utilities|Casting|CastToThrowable_Pistol OtherActor)
  (Effects|SpawnEmitteratLocation "/Game/StarterContent/Particles/P_Explosion.P_Explosion" _returnvalue)
  (Audio|PlaySoundatLocation "/Game/Sounds/StockAudio/Explosion02.Explosion02" _returnvalue)
  (Actor|DestroyActor))

(event EventBeginPlay
  ;[1 1 1] Set Patrol Points
  (Variables|Default|SetPatrol%20Points (Utilities|Array|MakeArray (Transformation|GetWorldLocation (Variables|Default|GetPatrol%20Point%201)) (Transformation|GetWorldLocation (Variables|Default|GetPatrol%20Point%202)) (Transformation|GetWorldLocation (Variables|Default|GetPatrol%20Point%203))))
  (CallFunction|GetRandomLocation)
  ;[1 1 1] Creates Spawns Gun in Hand Of Enemy
  (bind _returnvalue (Game|SpawnActorfromClass "/Game/Guns/Holdable_Pistol.Holdable_Pistol_C" (Math|Transform|MakeTransform "0, 0, 0" "0, 0, 0" "1.000000,1,1") "Undefined" 0 0))
  (Transformation|AttachComponentToComponent _returnvalue (Variables|Character|GetMesh) "GunHoldingBone" "KeepRelative" "KeepRelative" "KeepRelative" false))

(fn ConstructionScript)

(fn GetRandomLocation
  (Variables|Default|SetCurrentPatrolPoint (Math|Random|RandomInteger (Utilities|Array|Length (Variables|Default|GetPatrol%20Points)))))