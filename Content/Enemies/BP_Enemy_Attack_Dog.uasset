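; Attack dog enemy that wanders the navmesh until it sees the player, then sprints after them and deals damage on reaching them.
; PawnSensing sightings drive the chase, with a retriggerable delay clearing the seen flag and a MultiGate throttling the spotted sound.
; Overlapping a harmful Throwable_Gun costs health with explosion and hurt feedback; a hit at zero health destroys the dog and decrements the game instance's EnemiesLeft.
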(event OnSeePawn(PawnSensing)
  (params (Pawn :type Pawn%20Object%20Reference))
  ;[1 1 1] Chases Player
  (Variables|/Script/Engine.CharacterMovementComponent|SetMaxWalkSpeed (Variables|Character|GetCharacterMovement) 1e+03)
  (bind _asplayer_character (Utilities|Casting|CastToPlayerCharacter Pawn))
  (Variables|Default|SetcanSeePlayer true)
  (Utilities|FlowControl|Sequence
    (:then_0
      (AI|AIMoveTo self "0, 0, 0" _asplayer_character 5.0 false
        (:then
          (Utilities|FlowControl|RetriggerableDelay 1.0)
          (Variables|Default|SetcanSeePlayer false))
        (:OnSuccess
          (Default|Take5Damage _asplayer_character)
          (Utilities|FlowControl|Delay 0.5))))
    (:then_1
      (Utilities|FlowControl|MultiGate false false 0 :!label _label
        (:Out%200
          (Audio|PlaySoundatLocation "/Game/Sounds/Sound_Cues/Enemy_Spotted.Enemy_Spotted" (Transformation|GetActorLocation)))
        (:Out%201
          (Utilities|FlowControl|RetriggerableDelay 1e+01)
          (goto _label Reset))))))

(event Collision|EventActorBeginOverlap
  (params (OtherActor :type Actor%20Object%20Reference))
  (bind _returnvalue (Transformation|GetActorLocation))
  ;[1 1 1] Get damaged if hit/Dies if hit if Health = 0
  (bind _asthrowable_gun (Utilities|Casting|CastToThrowable_Gun OtherActor))
  (if (Variables|/Game/Guns/Throwable_Pistol.Throwable_Pistol_C|GetcanHurtEnemies _asthrowable_gun)
    (if (<= (Variables|Default|GetHealth) 0.0)
      (Effects|SpawnEmitteratLocation "/Game/StarterContent/Particles/P_Explosion.P_Explosion" _returnvalue)
      (Audio|PlaySoundatLocation "/Game/Sounds/Sound_Cues/Enemy_Hurt.Enemy_Hurt" _returnvalue)
      (bind _aswna_game_instance (Utilities|Casting|CastToWNA_Game_Instance (Game|GetGameInstance)))
      (Math|Integer|DecrementInt (Variables|/Game/GameManagement/WNA_Game_Instance.WNA_Game_Instance_C|GetenemiesLeft _aswna_game_instance)
        (:%20%20
          (Actor|DestroyActor)))
      (else
        (Variables|Default|SetHealth (- (Variables|Default|GetHealth) 5.0))
        (Effects|SpawnEmitteratLocation "/Game/StarterContent/Particles/P_Explosion.P_Explosion" _returnvalue) ; for now all that can be done is explosion : to add other effects must\n make a class to spawn them and spawn object of that class so it can be\n destroyed
        (Audio|PlaySoundatLocation "/Game/Sounds/Sound_Cues/Enemy_Hurt.Enemy_Hurt" _returnvalue)))))

(event EventTick
  (params (DeltaSeconds :type Float%20%28single-precision%29))
  ;[1 1 1] Wanders
  (if (not (Variables|Default|GetcanSeePlayer))
    (Variables|/Script/Engine.CharacterMovementComponent|SetMaxWalkSpeed (Variables|Character|GetCharacterMovement) 2e+02)
    (if (not (Variables|Default|Getwandering))
      (bind _outactors (Actor|GetAllActorsOfClass "/Script/Engine.RecastNavMesh"))
      (AI|AIMoveTo self (.RandomLocation (Class|NavigationSystem|GetRandomPointinNavigableRadius (Transformation|GetActorLocation) 1e+03 (Utilities|Array|Get(acopy) _outactors))) 0 5.0 false
        (:then
          (Variables|Default|Setwandering true))
        (:OnSuccess
          (Variables|Default|Setwandering false :!label _label))
        (:OnFail
          (goto _label))))))

(fn ConstructionScript)