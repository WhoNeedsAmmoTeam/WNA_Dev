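; Patrolling enemy that wanders the navmesh, throws pistols at the player and explodes when hit by a thrown pistol.
; Tick drives random AIMoveTo wandering until PawnSensing spots the player and sets CanSeePlayer, which this graph never clears.
; On sight it faces the player and, if SpawnProjectile is set, launches a spinning pistol with impulses, then keeps repositioning to random nearby points.
; Any overlapping Throwable_Pistol destroys it outright, with damage handling marked as to-do.
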(event OnSeePawn(PawnSensing)
  (params (Pawn :type Pawn%20Object%20Reference))
  ;[1 1 1] Shoot Logic
  (Variables|Default|SetCan%20See%20Player true)
  (bind _asplayer_character (Utilities|Casting|CastToPlayerCharacter Pawn))
  (Utilities|FlowControl|Sequence
    (:then_0
      (Transformation|SetActorRotation (Math|Rotator|FindLookatRotation (Transformation|GetActorLocation) (Transformation|GetActorLocation _asplayer_character))))
    (:then_1
      (if (Variables|Default|GetSpawnProjectile)
        (bind _returnvalue (Game|SpawnActorfromClass "/Game/Guns/Throwable_Pistol_ENEMY.Throwable_Pistol_ENEMY_C" (Transformation|GetWorldTransform (Variables|Default|GetGunSpawnLocation)) "Undefined" 0 0))
        (Physics|AddImpulse (Variables|/Game/Guns/Throwable_Pistol_ENEMY.Throwable_Pistol_ENEMY_C|GetStaticMesh _returnvalue) (* (Math|Vector|GetForwardVector (Variables|Default|GetGunSpawnLocation)) 2.5e+03) "None" true)
        (Class|PrimitiveComponent|AddAngularImpulse (Variables|/Game/Guns/Throwable_Pistol_ENEMY.Throwable_Pistol_ENEMY_C|GetStaticMesh _returnvalue) (* (Math|Random|RandomUnitVector) 3e+01) "None" true)
        (Audio|PlaySoundatLocation "/Game/Sounds/Sound_Cues/Throw_Enemy.Throw_Enemy" (Transformation|GetActorLocation))
        (Components|Animation|PlayAnimation (Variables|Character|GetMesh) "/Game/PlayerCharacter/Animation/Animations/throwing.throwing" false)
        (Utilities|FlowControl|Delay 2.5)
        (bind _outactors (Actor|GetAllActorsOfClass "/Script/Engine.RecastNavMesh" :!label _label))
        (AI|AIMoveTo self (.RandomLocation (Class|NavigationSystem|GetRandomPointinNavigableRadius (Transformation|GetActorLocation) 1e+03 (Utilities|Array|Get(acopy) _outactors))) 0 5.0 false
          (:then
            (Utilities|FlowControl|RetriggerableDelay 1.0)
            (if (Variables|Default|GetCan%20See%20Player)
              (goto _label))))))))

(event Collision|EventActorBeginOverlap
  (params (OtherActor :type Actor%20Object%20Reference))
  (bind _returnvalue (Transformation|GetActorLocation))
  ;[1 1 1] Dies If Hit [CHANGE TO TAKE DMG]
  (Utilities|Casting|CastToThrowable_Pistol OtherActor)
  (Effects|SpawnEmitteratLocation "/Game/StarterContent/Particles/P_Explosion.P_Explosion" _returnvalue)
  (Audio|PlaySoundatLocation "/Game/Sounds/StockAudio/Explosion02.Explosion02" _returnvalue)
  (Actor|DestroyActor))

(event EventTick
  (params (DeltaSeconds :type Float%20%28single-precision%29))
  ;[1 1 1] Wandering
  (if (not (Variables|Default|GetCan%20See%20Player))
    (Variables|/Script/Engine.CharacterMovementComponent|SetMaxWalkSpeed (Variables|Character|GetCharacterMovement) 4e+02)
    (if (not (Variables|Default|GetIsWandering))
      (bind _outactors (Actor|GetAllActorsOfClass "/Script/Engine.RecastNavMesh"))
      (AI|AIMoveTo self (.RandomLocation (Class|NavigationSystem|GetRandomPointinNavigableRadius (Transformation|GetActorLocation) 1e+03 (Utilities|Array|Get(acopy) _outactors))) 0 5.0 false
        (:then
          (Variables|Default|SetIsWandering true))
        (:OnSuccess
          (Variables|Default|SetIsWandering false :!label _label))
        (:OnFail
          (goto _label)))
      (Utilities|FlowControl|Delay 0.5))))

(fn ConstructionScript)