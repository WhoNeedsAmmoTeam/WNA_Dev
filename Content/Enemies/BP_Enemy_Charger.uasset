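; Charger enemy that wanders, rushes the player on sight and explodes when hit by a thrown pistol.
; While the player is unseen, Tick lowers fly speed and chains AI moves to random navmesh points.
; PawnSensing raises speed and starts a chase that damages the player on arrival, with a retriggerable delay clearing the sighted flag.
; Overlapping a Throwable_Pistol spawns explosion effects and sound, then destroys the actor.
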(event OnSeePawn(PawnSensing)
  (params (Pawn :type Pawn%20Object%20Reference))
  ;[1 1 1] Chases Player
  (Variables|/Script/Engine.CharacterMovementComponent|SetMaxFlySpeed (Variables|Character|GetCharacterMovement) 7.5e+02)
  (bind _asplayer_character (Utilities|Casting|CastToPlayerCharacter Pawn))
  (Variables|Default|SetcanSeePlayer true)
  (AI|AIMoveTo self "0, 0, 0" _asplayer_character 5.0 false
    (:then
      (Utilities|FlowControl|RetriggerableDelay 0.5)
      (Variables|Default|SetcanSeePlayer false))
    (:OnSuccess
      (Default|Take5Damage _asplayer_character)
      (Utilities|FlowControl|Delay 0.5))))

(event Collision|EventActorBeginOverlap
  (params (OtherActor :type Actor%20Object%20Reference))
  (bind _returnvalue (Transformation|GetActorLocation))
  ;[1 1 1] Dies If Hit
  (Utilities|Casting|CastToThrowable_Pistol OtherActor)
  (Effects|SpawnEmitteratLocation "/Game/StarterContent/Particles/P_Explosion.P_Explosion" _returnvalue)
  (Audio|PlaySoundatLocation "/Game/Sounds/StockAudio/Explosion02.Explosion02" _returnvalue)
  (Actor|DestroyActor))

(event EventTick
  (params (DeltaSeconds :type Float%20%28single-precision%29))
  ;[1 1 1] Wanders
  (if (not (Variables|Default|GetcanSeePlayer))
    (Variables|/Script/Engine.CharacterMovementComponent|SetMaxFlySpeed (Variables|Character|GetCharacterMovement) 2.5e+02)
    (if (not (Variables|Default|Getwandering))
      (bind _outactors (Actor|GetAllActorsOfClass "/Script/Engine.RecastNavMesh"))
      (AI|AIMoveTo self (.RandomLocation (Class|NavigationSystem|GetRandomPointinNavigableRadius (Transformation|GetActorLocation) 1e+03 (Utilities|Array|Get(acopy) _outactors))) 0 5.0 false
        (:then
          (Variables|Default|Setwandering true))
        (:OnSuccess
          (Variables|Default|Setwandering false :!label _label))
        (:OnFail
          (goto _label))))))

(fn ConstructionScript)