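; Enemy that turns to face a sensed player character, throws spinning pistol projectiles and dies on contact with a Throwable_Pistol.
; PawnSensing drives aiming and firing, with impulses applied to the spawned mesh and a half-second Delay gating throws.
; Overlapping a Throwable_Pistol triggers an explosion effect and sound, then destroys the enemy.
; BeginPlay picks one of three patrol points, but the timeline that lerps toward them never runs.
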(event OnSeePawn(PawnSensing)
  (params (Pawn :type Pawn%20Object%20Reference))
  ;[1 1 1] Move and Shoot Logic
  (bind _asplayer_character (Utilities|Casting|CastToPlayerCharacter Pawn))
  (Utilities|FlowControl|Sequence
    (:then_0
      (Transformation|SetActorRotation (Math|Rotator|FindLookatRotation (Transformation|GetActorLocation) (Transformation|GetActorLocation _asplayer_character))))
    (:then_1
      (if (Variables|Default|GetSpawnProjectile)
        (bind _returnvalue (Game|SpawnActorfromClass "/Game/Guns/Throwable_Pistol_ENEMY.Throwable_Pistol_ENEMY_C" (Transformation|GetWorldTransform (Variables|Default|GetProjectileSpawnLocation)) "Undefined" 0 0))
        (Physics|AddImpulse (Variables|/Game/Guns/Throwable_Pistol_ENEMY.Throwable_Pistol_ENEMY_C|GetStaticMesh _returnvalue) (* (Math|Vector|GetForwardVector (Variables|Default|GetBase)) 2.5e+03) "None" true)
        (Class|PrimitiveComponent|AddAngularImpulse (Variables|/Game/Guns/Throwable_Pistol_ENEMY.Throwable_Pistol_ENEMY_C|GetStaticMesh _returnvalue) (* (Math|Random|RandomUnitVector) 3e+01) "None" true)
        (Audio|PlaySoundatLocation "/Game/Sounds/Sound_Cues/Throw_Enemy.Throw_Enemy" (Transformation|GetActorLocation))
        (Variables|Default|SetSpawnProjectile false)
        (Utilities|FlowControl|Delay 0.5)
        (Variables|Default|SetSpawnProjectile true)))))

(event EventBeginPlay
  ;[1 1 1] Set Patrol Points
  (Variables|Default|SetPatrolPoints (Utilities|Array|MakeArray (Transformation|GetWorldLocation (Variables|Default|GetMovePosition1)) (Transformation|GetWorldLocation (Variables|Default|GetMovePosition2)) (Transformation|GetWorldLocation (Variables|Default|GetMovePosition3))))
  (CallFunction|GetRandomLocation))

(event Collision|EventActorBeginOverlap
  (params (OtherActor :type Actor%20Object%20Reference))
  (bind _returnvalue (Transformation|GetActorLocation))
  ;[1 1 1] Kills Enemy if Hit
  (Utilities|Casting|CastToThrowable_Pistol OtherActor)
  (Effects|SpawnEmitteratLocation "/Game/StarterContent/Particles/P_Explosion.P_Explosion" _returnvalue)
  (Audio|PlaySoundatLocation "/Game/Sounds/StockAudio/Explosion02.Explosion02" _returnvalue)
  (Actor|DestroyActor))

(fn ConstructionScript)

(fn GetRandomLocation
  (Variables|Default|SetCurrentPatrolPoint (Math|Random|RandomInteger (Utilities|Array|Length (Variables|Default|GetPatrolPoints)))))